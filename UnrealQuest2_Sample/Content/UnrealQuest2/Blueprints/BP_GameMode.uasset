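; Game mode for an UnrealQuest2 stage that keeps the total score and handles goal clear and level restart.
; AddScore accumulates points, and Tick prints the running score on screen each frame.
; ShowUpResult stops Tick, shows the mouse cursor, disables character input and calls the restart immediately, with no result screen.
; Restart reloads the current level through the RestartLevel console command, intended for a single-stage game.
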(event Custom|AddScore
  (params (AddValue :type Integer))
  ;[1 1 1] 初級：「アイテムゲットしたらスコアが増える仕組み」合計値への加算
  (Variables|Default|SetTotalScore (+ (Variables|Default|GetTotalScore) AddValue)))

(event Custom|ShowUpResult
  (bind _returnvalue (Game|GetPlayerController 0))
  ;[1 0.2543 0] ゴール到着時のクリア処理
  (Actor|Tick|SetActorTickEnabled false :!pinned true) ; Tickを無効化して制限時間周りの処理を停止
  ;;[1 1 1] マウスカーソルの表示、キャラクターへの入力の無効化(移動など)
  (Variables|/Script/Engine.PlayerController|SetbShowMouseCursor _returnvalue true)
  (Input|DisableInput (Game|GetPlayerCharacter 0) _returnvalue)
  (CallFunction|RestartGameUQ))

(event Custom|RestartGame_UQ
  ;[1 1 1] ゲームのリスタート
  (Development|ExecuteConsoleCommand "RestartLevel" 0 :!pinned true) ; 1ステージだけの場合はこれでOK
)

(event EventTick
  (params (DeltaSeconds :type Float%20%28single-precision%29))
  (Development|PrintString (Utilities|String|Append "スコア : " (Utilities|String|ToString(Integer) (Variables|Default|GetTotalScore))) true true "(R=0.000000,G=0.660000,B=1.000000,A=1.000000)" (Utilities|Time|GetWorldDeltaSeconds)))

(event EventBeginPlay
  (Development|PrintString "スタート！" true true "(R=0.000000,G=0.660000,B=1.000000,A=1.000000)" 5.0))

(fn ConstructionScript)